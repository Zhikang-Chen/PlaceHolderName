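; BP_Tower is a tower actor for the zombie game that tracks and faces a target.
; AttackTarget picks the closest actor from the AllTarget array and stores it as CurrentTarget.
; Each Tick rotates the Scene component toward CurrentTarget's location while it is valid.
; Nothing in this graph fills AllTarget, calls AttackTarget or deals damage, so it only handles target selection and aiming.
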(event EventBeginPlay)

(event Collision|EventActorBeginOverlap
  (params (OtherActor :type Actor%20Object%20Reference)))

(event EventTick
  (params (DeltaSeconds :type Float%20%28single-precision%29))
  (bind _currenttarget (Variables|Default|GetCurrentTarget))
  (Utilities|IsValid _currenttarget
    (:Is%20Valid
      (Class|CPPActorUtilities|RotateActorComponentto (Variables|Default|GetScene) (Transformation|GetActorLocation _currenttarget)))))

(event EventAttackTarget
  (bind _alltarget (Variables|Default|GetAllTarget))
  (if (not (Utilities|Array|IsEmpty _alltarget))
    (bind _returnvalue (Class|CPPActorUtilities|GetClosestActorfromArray self _alltarget))
    (Utilities|IsValid _returnvalue
      (:Is%20Valid
        (Variables|Default|SetCurrentTarget _returnvalue)))))

(fn ConstructionScript)