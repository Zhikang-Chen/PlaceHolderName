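; BP_Grid is a grid actor that snaps the player's mouse world position to grid coordinates.
; Every Tick it casts the player pawn to BP_PlayerCharacter, converts its MouseWorldLocation to a grid location and back, and writes the result to SnappadLocation.
; The conversion functions are called here but defined outside these graphs, and the debug prints and sphere are disconnected.
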(event EventBeginPlay)

(event Collision|EventActorBeginOverlap
  (params (OtherActor :type Actor%20Object%20Reference)))

(event EventTick
  (params (DeltaSeconds :type Float%20%28single-precision%29))
  (bind _asbp_player_character (Utilities|Casting|CastToBP_PlayerCharacter (Game|Player|GetPlayerPawn 0)))
  (Variables|/Game/Zombie/_Blueprints/PlayerCharacter/BP_PlayerCharacter.BP_PlayerCharacter_C|SetSnappadLocation _asbp_player_character (Class|CPPGrid|ConvertGridLocationtoWorldLocation (Class|CPPGrid|ConvertWorldLocationtoGridLocation (Variables|/Game/Zombie/_Blueprints/PlayerCharacter/BP_PlayerCharacter.BP_PlayerCharacter_C|GetMouseWorldLocation _asbp_player_character)))))

(fn ConstructionScript)